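; Grid actor that procedurally builds a rectangular room of floor tiles, border walls, corners and random doors on BeginPlay.
; Floor tiles are spawned by row and column into FloorTiles, then edge tiles call MakeWall to spawn inward-facing walls and unrotated corners into WallTiles.
; Up to MaxDoors random WallTiles entries, corners included, are swapped for doors, though the array removal re-rolls its index, so it can drop a different entry.
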(event `self.ReceiveBeginPlay`
  (bind (_returnvalue_x _returnvalue_y _returnvalue_z) (`KismetMathLibrary.BreakVector` (`self.K2_GetActorLocation`)))
  (bind _tilesize (`self.TileSize`))
  (bind _tilesize_2 (`self.TileSize`))
  (bind _tilesize_3 (`self.TileSize`))
  (bind _walltiles (`self.WallTiles`))
  (bind _item_tileclass (break `/Game/Grid/STRUCT_TIle` (`KismetArrayLibrary.Array_Get` _walltiles (`self.TempDoorIndex`))))
  (bind _returnvalue (* (`self.TileSize`) -1))
  (bind _returnvalue_2 (`KismetMathLibrary.RandomIntegerInRange` 0 (- (`KismetArrayLibrary.Array_Length` _walltiles) 1)))
  (`|ExecutionSequence`
    (:`then_0`
      ;[1 1 1] Create Floor
      (`KismetArrayLibrary.Array_Clear` (`self.FloorTiles`))
      (for _index (range (`self.X Tiles`))
        (bind _returnvalue_3 (`|SpawnActorFromClass` (`self.FloorClass`) (`KismetMathLibrary.MakeTransform` (`KismetMathLibrary.MakeVector` (+ (* _index (`KismetMathLibrary.Conv_IntToDouble` (`self.TileSize`))) _returnvalue_x) _returnvalue_y _returnvalue_z)) "Undefined" "OverrideRootScale"))
        (bind _structout (setmembers `/Game/Grid/STRUCT_TIle` :`StructRef` (`self.TempTile`) :`TileClass` _returnvalue_3 :`TileLocation` (`self.K2_GetActorLocation` _returnvalue_3) :`Row` _index :`Column` 0))
        (`KismetArrayLibrary.Array_Add` (`self.FloorTiles`) _structout)
        (for _index_2 (range 1 (`self.Y Tiles`))
          (bind (_returnvalue_x_2 _returnvalue_y_2 _returnvalue_z_2) (`KismetMathLibrary.BreakVector` (`self.K2_GetActorLocation` _returnvalue_3)))
          (bind _returnvalue_4 (`|SpawnActorFromClass` (`self.FloorClass`) (`KismetMathLibrary.MakeTransform` (`KismetMathLibrary.MakeVector` _returnvalue_x_2 (+ (* _index_2 (`KismetMathLibrary.Conv_IntToDouble` (`self.TileSize`))) _returnvalue_y_2) _returnvalue_z_2)) "Undefined" "OverrideRootScale"))
          (bind _structout_2 (setmembers `/Game/Grid/STRUCT_TIle` :`StructRef` (`self.TempTile`) :`TileClass` _returnvalue_4 :`TileLocation` (`self.K2_GetActorLocation` _returnvalue_4) :`Row` _index :`Column` _index_2))
          (`KismetArrayLibrary.Array_Add` (`self.FloorTiles`) _structout_2))))
    (:`then_1`
      (for _array_element (`self.FloorTiles`)
        ;[1 1 1] Create walls
        (`|ExecutionSequence`
          (:`then_0`
            (bind (_tileclass _tilelocation _row _column) (break `/Game/Grid/STRUCT_TIle` _array_element))
            (if (== _row 0)
              (`self.MakeWall` _tileclass (* (`self.TileSize`) -1) 0 (`self.WallClass`) true)))
          (:`then_1`
            (if (== _column 0)
              (`self.MakeWall` _tileclass 0 (* (`self.TileSize`) -1) (`self.WallClass`) true)))
          (:`then_2`
            (if (== _row (- (`self.X Tiles`) 1))
              (`self.MakeWall` _tileclass (`self.TileSize`) 0 (`self.WallClass`) true)))
          (:`then_3`
            (if (== _column (- (`self.Y Tiles`) 1))
              (`self.MakeWall` _tileclass 0 (`self.TileSize`) (`self.WallClass`) true)))
          (:`then_4`
            (if (and (== _row 0) (== _column 0))
              (`self.MakeWall` _tileclass _returnvalue _returnvalue (`self.CornerClass`))))
          (:`then_5`
            (if (and (== _row 0) (== _column (- (`self.Y Tiles`) 1)))
              (`self.MakeWall` _tileclass (* _tilesize_2 -1) _tilesize_2 (`self.CornerClass`))))
          (:`then_6`
            (if (and (== _column 0) (== _row (- (`self.X Tiles`) 1)))
              (`self.MakeWall` _tileclass _tilesize_3 (* _tilesize_3 -1) (`self.CornerClass`))))
          (:`then_7`
            (`KismetSystemLibrary.PrintString` (`KismetStringLibrary.Concat_StrStr` (`KismetStringLibrary.Conv_IntToString` _row) "-" (`KismetStringLibrary.Conv_IntToString` _column)))
            (if (and (== _row (- (`self.X Tiles`) 1)) (== _column (- (`self.Y Tiles`) 1)))
              (`self.MakeWall` _tileclass _tilesize _tilesize (`self.CornerClass`))))))
      (for _ (range 1 (+ (`self.MaxDoors`) 1))
        (set `self.TempDoorIndex` _returnvalue_2)
        (`|ExecutionSequence`
          (:`then_0`
            (bind _output_get (set `self.TempDoorTransform` (`SceneComponent.K2_GetComponentToWorld` (`/Game/Grid/BP_Tile.DefaultSceneRoot` _item_tileclass))))
            (bind _returnvalue_5 (`|SpawnActorFromClass` (`self.DoorClass`) _output_get "Undefined" "OverrideRootScale"))
            (bind _structout_3 (setmembers `/Game/Grid/STRUCT_TIle` :`StructRef` (`self.TempTile`) :`TileClass` _returnvalue_5 :`TileLocation` (0.0 0.0 0.0) :`Row` 0 :`Column` 0))
            (`KismetArrayLibrary.Array_Add` (`self.DoorTiles`) _structout_3))
          (:`then_1`
            (`self.K2_DestroyActor` _item_tileclass)
            (`KismetArrayLibrary.Array_Remove` _walltiles _returnvalue_2)))))))

(fn `MakeWall`
  (params (EdgeActor :type "/Game/Grid/BP_Tile Object Reference") (`X Offset` :type Integer) (`Y Offset` :type Integer) (TileClass :type "/Game/Grid/BP_Tile Class Reference") (bRotate :type Boolean))
  (bind _returnvalue (`|SpawnActorFromClass` TileClass (`KismetMathLibrary.MakeTransform` (`KismetMathLibrary.MakeVector` (+ (.x (`self.K2_GetActorLocation` EdgeActor)) (`KismetMathLibrary.Conv_IntToDouble` `X Offset`)) (+ (.y (`self.K2_GetActorLocation` EdgeActor)) (`KismetMathLibrary.Conv_IntToDouble` `Y Offset`)) (.z (`self.K2_GetActorLocation` EdgeActor)))) "Undefined" "OverrideRootScale"))
  (if bRotate
    (`self.SetActorRotation` _returnvalue (`KismetMathLibrary.FindLookAtRotation` (`self.K2_GetActorLocation` _returnvalue) (`self.K2_GetActorLocation` EdgeActor))))
  (bind _structout (setmembers `/Game/Grid/STRUCT_TIle` :`StructRef` (`self.TempTile`) :`TileClass` _returnvalue :`TileLocation` (`self.K2_GetActorLocation` _returnvalue) :`Row` 0 :`Column` 0))
  (`KismetArrayLibrary.Array_Add` (`self.WallTiles`) _structout)
  (return))

(fn `UserConstructionScript`)