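; Unfinished pathfinder Blueprint whose Action event scans all BP_Tile actors for the one occupied by an AiController.
; A match triggers nothing, and an unoccupied tile wires back into the loop's start rather than continuing to the next element.
; Disconnected nodes hint at intended use of surrounding tiles and a direction toward the player pawn, alongside an empty, unreachable loop over AI controllers.
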(event `Action`
  (bind _outactors (`GameplayStatics.GetAllActorsOfClass` "/Game/Grid/BP_Tile.BP_Tile_C"))
  (for _array_element _outactors :!label _label
    (if (`/Game/Grid/BP_Tile.bOccupied` _array_element)
      (if (== (`/Game/Grid/BP_Tile.occupant` _array_element) (`self.aiController`))
        _)
      (else
        (goto _label)))))

(fn `UserConstructionScript`)