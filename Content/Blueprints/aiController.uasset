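; Turn-based enemy AI actor that seeks or attacks the player through a simple state machine.
; Action checks player distance: beyond range in Seek opens a gate, never closed here, letting Tick run PathFinder actors' Action and clear Turn.
; Within range in Fight, a random roll either damages PlayerPawn or misses, then clears Turn.
; deadState destroys the actor at zero or lower Health when its Seek variable equals Die.
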(event `deadState`
  ;[1 1 1] Dead State
  (`/Engine/EditorBlueprintResources/StandardMacros.CompareInt` (`self.health`)
    (:`==`
      _)
    (:`<`
      _))
  (if true
    (switch `/Game/Blueprints/ENUM_AIState` "NewEnumerator0"
      (:`NewEnumerator2`
        (`self.K2_DestroyActor` self)))))

(event `self.ReceiveTick`
  (params (DeltaSeconds :type "Float (single-precision)"))
  ;[1 1 1] Seek
  (`/Engine/EditorBlueprintResources/StandardMacros.Gate` true :!label _label
    (:`Exit`
      (bind _outactors (`GameplayStatics.GetAllActorsOfClass` "/Game/Blueprints/pathFinder.pathFinder_C"))
      (`/Game/Blueprints/pathFinder.Action` _outactors)
      (set `self.bTurn` false))))

(event `Action`
  ;[1 1 1] FSM
  (`/Engine/EditorBlueprintResources/StandardMacros.CompareFloat` (`self.GetDistanceTo` self (`self.K2_GetPawn` (`GameplayStatics.GetPlayerController` 0))) 450.0
    (:`>`
      ;[1 1 1] Seek
      (switch `/Game/Blueprints/ENUM_AIState` (`self.State`)
        (:`NewEnumerator0`
          (goto _label :!via `Open`))))
    (:`==`
      _)
    (:`<`
      _))
  (switch `/Game/Blueprints/ENUM_AIState` (`self.State`)
    (:`NewEnumerator1`
      ;[1 1 1] Fight State
      (switch `int` (`KismetMathLibrary.RandomInteger` 10)
        (:`0`
          _)
        (:`1`
          _)
        (:`2`
          _)
        (:`3`
          _)
        (:`4`
          (bind _outactors (`GameplayStatics.GetAllActorsOfClass` "/Game/PlayerPawn.PlayerPawn_C" :!label _label_2))
          (`/Game/PlayerPawn.TakeDamage` (`KismetArrayLibrary.Array_Get` _outactors) 10))
        (:`5`
          (goto _label_2))
        (:`6`
          (goto _label_2))
        (:`7`
          (goto _label_2))
        (:`8`
          (goto _label_2))
        (:`9`
          (goto _label_2))
        (:`10`
          (goto _label_2)))
      (set `self.bTurn` false))))

(fn `UserConstructionScript`)