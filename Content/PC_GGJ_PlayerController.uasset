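; Player controller for a game jam game that moves the possessed pawn between tiles.
; MoveToTile turns the control rotation to face the target, then plays a timeline that teleports the pawn toward it with a per-update lerp from its current position.
; A second timeline track lerps the PlayerPawn mesh's relative rotation between zero and a yaw or pitch offset as it moves.
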(event `MoveToTile`
  (params (NewLocation :type "Vector Structure"))
  (bind _returnvalue (`self.K2_GetPawn` self))
  (`self.SetControlRotation` (`KismetMathLibrary.FindLookAtRotation` (`self.K2_GetActorLocation` (`self.K2_GetPawn`)) NewLocation))
  (bind (_direction _newtrack_0 _newtrack_1) (`Timeline|Move` :!via `PlayFromStart`)
    (:`Update`
      (`|ExecutionSequence`
        (:`then_0`
          (`self.K2_SetActorLocation` _returnvalue (`KismetMathLibrary.VLerp` (`self.K2_GetActorLocation` _returnvalue) NewLocation _newtrack_0) false true))
        (:`then_1`
          (bind _asplayer_pawn (cast `/Game/PlayerPawn` _returnvalue))
          (`SceneComponent.K2_SetRelativeRotation` (`/Game/PlayerPawn.SM_Player` _asplayer_pawn) (`KismetMathLibrary.RLerp` (struct) (struct :`Pitch` 30.0) _newtrack_1) false false))))))

(fn `UserConstructionScript`)