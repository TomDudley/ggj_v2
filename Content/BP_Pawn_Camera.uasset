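; BP_Pawn_Camera is an actor, apparently a camera rig, that positions itself on the PlayerPawn.
; After a short delay at BeginPlay it jumps to the first PlayerPawn found in the level.
; Its CatchUp event finds that pawn again and plays the Catch timeline, lerping from the rig's current location toward the pawn's live location on each update.
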(event `self.ReceiveBeginPlay`
  (`KismetSystemLibrary.Delay` 0.2)
  (bind _outactors (`GameplayStatics.GetAllActorsOfClass` "/Game/PlayerPawn.PlayerPawn_C"))
  (`self.K2_SetActorLocation` (`self.K2_GetActorLocation` (`KismetArrayLibrary.Array_Get` _outactors))))

(event `CatchUp`
  (bind _outactors (`GameplayStatics.GetAllActorsOfClass` "/Game/PlayerPawn.PlayerPawn_C"))
  (set `self.Figure` (`KismetArrayLibrary.Array_Get` _outactors))
  (bind (_direction _newtrack_1) (`Timeline|Catch` :!via `PlayFromStart`)
    (:`Update`
      (`self.K2_SetActorLocation` (`KismetMathLibrary.VLerp` (`self.K2_GetActorLocation`) (`self.K2_GetActorLocation` (`self.Figure`)) _newtrack_1)))))

(fn `UserConstructionScript`)