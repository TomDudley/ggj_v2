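; BP_CameraController is a player controller that handles turn-gated, click-to-move input for a PlayerPawn figurine.
; Clicks trace from the camera to the cursor's projection on the Z=0 plane.
; Floor tiles trigger a timeline move, then the camera pawn's CatchUp; doors restart the level.
; Floor moves and nearby chest clicks end the turn, which nothing here restores.
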(event `self.ReceiveBeginPlay`
  (`KismetSystemLibrary.Delay` 0.2)
  (bind _outactors (`GameplayStatics.GetAllActorsOfClass` "/Game/PlayerPawn.PlayerPawn_C"))
  (set `self.Figurine` (`KismetArrayLibrary.Array_Get` _outactors))
  (set `self.IsMyTurn` true))

(event `Key|LeftMouseButton`
  (params (Key :type "Key Structure" :default "AnyKey"))
  (bind (_worldlocation _worlddirection) (`self.DeprojectMousePositionToWorld` self))
  ;[1 1 1] Left Mouse Clicked
  (:`Pressed`
    (if (`self.IsMyTurn`)
      (bind _outhit (`KismetSystemLibrary.LineTraceSingle` (`self.K2_GetActorLocation` (`PlayerController.PlayerCameraManager` (`GameplayStatics.GetPlayerController` 0))) (+ _worldlocation (* (* _worlddirection (/ (.z _worldlocation) (.z _worlddirection))) -1.0)) "TraceTypeQuery1"))
      (bind (_bblockinghit _binitialoverlap _time _location _impactpoint _normal _impactnormal _physmat _hitactor) (`GameplayStatics.BreakHitResult` _outhit))
      (bind _returnvalue (`GameplayStatics.GetObjectClass` _hitactor))
      (if (== _returnvalue "/Game/Grid/BP_Tile_Floor.BP_Tile_Floor_C")
        (bind _returnvalue_2 (`self.K2_GetActorLocation` _hitactor))
        (`self.MoveToTile` _returnvalue_2)
        (set `self.IsMyTurn` false)
        (elif (== _returnvalue "/Game/BP_GoalChest.BP_GoalChest_C")
          (if (<= (`KismetMathLibrary.VSize` (- _returnvalue_2 (`self.K2_GetActorLocation` (`self.Figurine`)))) 200.0)
            (set `self.IsMyTurn` false))
          (elif (== _returnvalue "/Game/Grid/BP_Tile_Door.BP_Tile_Door_C")
            (`KismetSystemLibrary.ExecuteConsoleCommand` "RestartLevel")))))))

(event `MoveToTile`
  (params (NewLocation :type "Vector Structure"))
  (bind _figurine (`self.Figurine`))
  (bind _figurine_2 (`self.Figurine`))
  (`self.SetActorRotation` _figurine_2 (`KismetMathLibrary.FindLookAtRotation` (`self.K2_GetActorLocation` _figurine_2) NewLocation))
  (bind (_direction _newtrack_0) (`Timeline|Timeline_0` :!via `PlayFromStart`)
    (:`Update`
      (`|ExecutionSequence`
        (:`then_0`
          (`self.K2_SetActorLocation` _figurine (`KismetMathLibrary.VLerp` (`self.K2_GetActorLocation` _figurine) NewLocation _newtrack_0) false true))))
    (:`Finished`
      (bind _asbp_pawn_camera (cast `/Game/BP_Pawn_Camera` (`self.K2_GetPawn`)))
      (`/Game/BP_Pawn_Camera.CatchUp` _asbp_pawn_camera))))

(fn `UserConstructionScript`)